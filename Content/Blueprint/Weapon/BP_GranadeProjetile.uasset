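; BP_GranadeProjetile is a grenade projectile actor that explodes on a one-second fuse after spawning, then destroys itself.
; The explosion spawns a particle effect and applies radial damage around its location, crediting the instigator's controller, and draws a debug sphere showing the damage radius.
; Hits on its sphere component only spawn a rifle impact effect and do not trigger the explosion.
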(event `self.ReceiveBeginPlay`
  (`KismetSystemLibrary.Delay` 1.0)
  (`self.Explode`)
  (`self.K2_DestroyActor`))

(event `Explode`
  (bind _returnvalue (`self.K2_GetActorLocation`))
  (`GameplayStatics.SpawnEmitterAtLocation` "/Game/WeaponEffects/Explosion/P_Explosion.P_Explosion" _returnvalue)
  (`GameplayStatics.ApplyRadialDamage` :`BaseDamage` 100.0 :`Origin` _returnvalue :`DamageRadius` (`self.Damage Radius`) :`DamageCauser` self :`InstigatedByController` (`self.GetInstigatorController`))
  (`KismetSystemLibrary.DrawDebugSphere` _returnvalue (`self.Damage Radius`) 12 (struct :`R` 1.0 :`G` 0.87442 :`A` 1.0) 1.0 1.0))

(event `self.Sphere.OnComponentHit`
  (params (HitComponent :type "PrimitiveComponent Object Reference") (OtherActor :type "Actor Object Reference") (OtherComp :type "PrimitiveComponent Object Reference") (NormalImpulse :type "Vector Structure") (Hit :type "HitResult Structure (by ref)"))
  (`GameplayStatics.SpawnEmitterAtLocation` "/Game/WeaponEffects/GenericImpact/P_RifleImpact.P_RifleImpact" (`self.K2_GetActorLocation`)))

(fn `UserConstructionScript`)